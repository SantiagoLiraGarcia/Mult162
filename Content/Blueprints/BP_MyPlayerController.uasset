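; Player controller that drives the player's BP_MyCharacter from Enhanced Input actions.
; On BeginPlay it casts player character 0 and caches the reference for all input handlers.
; Jump calls the character's jump, Look adds yaw and pitch controller input, and PlayerMovement moves along the character's right and forward vectors.
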(event Input|EnhancedActionEvents|EnhancedInputActionIA_Jump
  (params (ActionValue :type Boolean) (ElapsedSeconds :type Float%20%28double-precision%29) (TriggeredSeconds :type Float%20%28double-precision%29) (InputAction :type Input%20Action%20Object%20Reference :default "/Game/Inputs/IA_Jump.IA_Jump"))
  (Character|Jump (Variables|Default|GetAs%20BP%20My%20Character)))

(event Input|EnhancedActionEvents|EnhancedInputActionIA_Look
  (params (ActionValue :type Vector%202D%20Structure) (ElapsedSeconds :type Float%20%28double-precision%29) (TriggeredSeconds :type Float%20%28double-precision%29) (InputAction :type Input%20Action%20Object%20Reference :default "/Game/Inputs/IA_Look.IA_Look"))
  (bind _as_bp_my_character (Variables|Default|GetAs%20BP%20My%20Character))
  (Pawn|Input|AddControllerYawInput _as_bp_my_character (.x ActionValue))
  (Pawn|Input|AddControllerPitchInput _as_bp_my_character (.y ActionValue)))

(event Input|EnhancedActionEvents|EnhancedInputActionIA_PlayerMovement
  (params (ActionValue :type Vector%202D%20Structure) (ElapsedSeconds :type Float%20%28double-precision%29) (TriggeredSeconds :type Float%20%28double-precision%29) (InputAction :type Input%20Action%20Object%20Reference :default "/Game/Inputs/IA_PlayerMovement.IA_PlayerMovement"))
  (bind _as_bp_my_character (Variables|Default|GetAs%20BP%20My%20Character))
  (Pawn|Input|AddMovementInput _as_bp_my_character (Transformation|GetActorRightVector _as_bp_my_character) (.x ActionValue) false)
  (Pawn|Input|AddMovementInput _as_bp_my_character (Transformation|GetActorForwardVector _as_bp_my_character) (.y ActionValue) false))

(event EventBeginPlay
  (bind _asbp_my_character (Utilities|Casting|CastToBP_MyCharacter (Game|GetPlayerCharacter 0)))
  (Variables|Default|SetAs%20BP%20My%20Character _asbp_my_character))

(fn ConstructionScript)