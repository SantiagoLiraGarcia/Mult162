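; BP_AnimDoor is a door the player swings open with the IA_Interact input, which BeginPlay enables on the actor.
; Interact checks the player character against the sphere's begin-overlap OtherActor, with no end-overlap handling.
; A DoOnce that is never reset then stores the starting rotation and plays a timeline that subtracts its track value from the whole actor's yaw, so the door opens once and never closes.
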(event OnComponentBeginOverlap(Sphere)
  (params (OverlappedComponent :type Primitive%20Component%20Object%20Reference) (OtherActor :type Actor%20Object%20Reference) (OtherComp :type Primitive%20Component%20Object%20Reference) (OtherBodyIndex :type Integer) (bFromSweep :type Boolean) (SweepResult :type Hit%20Result%20Structure%20%28by%20ref%29)))

(event Input|EnhancedActionEvents|EnhancedInputActionIA_Interact
  (params (ActionValue :type Boolean) (ElapsedSeconds :type Float%20%28double-precision%29) (TriggeredSeconds :type Float%20%28double-precision%29) (InputAction :type Input%20Action%20Object%20Reference :default "/Game/Inputs/IA_Interact.IA_Interact"))
  (if (== (Game|GetPlayerCharacter 0) (stale OnComponentBeginOverlap(Sphere) OtherActor))
    (Utilities|FlowControl|DoOnce false
      (:Completed
        (Development|PrintString "Interacting")
        (bind _output_get (Variables|Default|SetInitial%20Door%20Rotation (Transformation|GetActorRotation)))
        (bind _open_door_track (Timeline|Door%20Open%20Timeline Play)
          (:Update
            (Transformation|SetActorRotation (Math|Rotator|MakeRotator (.Roll (Math|Rotator|BreakRotator _output_get)) (.Pitch (Math|Rotator|BreakRotator _output_get)) (- (.Yaw (Math|Rotator|BreakRotator _output_get)) _open_door_track)))))))))

(event EventBeginPlay
  (Input|EnableInput (Game|GetPlayerController 0)))

(fn ConstructionScript)